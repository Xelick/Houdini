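; Blueprint function library of global helpers for save keys, checkpoints, pausing, mouse cursor, HUD access, floating text and sublevel names.
; Save and checkpoint calls forward to BP_CustomGameInstance, and HUD getters cast player 0's HUD, mostly printing errors on failure.
; CreateFloatingText spawns a UI_FloatingText widget, colored by type for damage, heals and blocked actions.
; GetCustomGameMode duplicates GetCustomGameInstance, returning the game instance despite its name.
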(fn SetSaveKeyData
  (params (Key :type String%20%28by%20ref%29) (Value :type Integer%20%28by%20ref%29))
  (Default|SetSaveKey (Game|GetCustomGameInstance) Key Value))

(fn GetSaveKeyData
  (params (Key :type String%20%28by%20ref%29))
  (return (Default|GetSaveKey (Game|GetCustomGameInstance) Key false)))

(fn SetCurrentCheckpointID
  (params (newId :type Integer) (isAllowingBacktrackingId :type Boolean))
  (Default|SetCheckpointID (Game|GetCustomGameInstance) newId isAllowingBacktrackingId))

(fn GetCurrentCheckpointID
  (return (Default|GetCheckpointID (Game|GetCustomGameInstance))))

(fn PauseGame
  (Game|SetGamePaused 0 true))

(fn ResumeGame
  (Game|SetGamePaused 0 false))

(fn ShowMouseCursor
  (Variables|/Script/Engine.PlayerController|SetbShowMouseCursor (Game|GetPlayerController 0) true))

(fn HideMouseCursor
  (Variables|/Script/Engine.PlayerController|SetbShowMouseCursor (Game|GetPlayerController 0) false))

(fn GetBaseCustomHUD
  (bind _ashud_base_custom (Utilities|Casting|CastToHUD_BaseCustom (HUD|GetHUD (Game|GetPlayerController 0))))
  (return _ashud_base_custom))

(fn CreateFloatingText
  (params (Text :type String) (TargetLocation :type Vector) (FloatingTextType :type EN_FloatingTextType%20Enum :default "NewEnumerator0") (Playback%20Speed :type Float%20%28single-precision%29))
  (bind _returnvalue (UserInterface|CreateWidget "/Game/Blueprints/Game/UI/Widgets/FloatingText/UI_FloatingText.UI_FloatingText_C" 0 Text TargetLocation (Game|GetPlayerController 0) (FloatingText|GetFloatingTextColor FloatingTextType) Playback%20Speed))
  (UserInterface|Viewport|AddtoViewport _returnvalue 0))

(fn GetFloatingTextColor
  (params (FloatingTextType :type EN_FloatingTextType%20Enum :default "NewEnumerator0"))
  (switch Utilities|FlowControl|Switch|SwitchonEN_FloatingTextType FloatingTextType
    (:NewEnumerator2
      (LocalVariables|SetFloatingTextColor "(R=1.000000,G=1.000000,B=1.000000,A=1.000000)"))
    (:NewEnumerator0
      (LocalVariables|SetFloatingTextColor "(R=1.000000,G=1.000000,B=1.000000,A=1.000000)"))
    (:NewEnumerator4
      (LocalVariables|SetFloatingTextColor "(R=1.000000,G=0.872354,B=0.000000,A=1.000000)"))
    (:NewEnumerator3
      (LocalVariables|SetFloatingTextColor "(R=1.000000,G=0.000000,B=0.000000,A=1.000000)"))
    (:NewEnumerator1
      (LocalVariables|SetFloatingTextColor "(R=0.000000,G=1.000000,B=0.019322,A=1.000000)"))
    (:NewEnumerator5
      (LocalVariables|SetFloatingTextColor "(R=0.171875,G=0.161436,B=0.166823,A=1.000000)")))
  (return (LocalVariables|GetFloatingTextColor)))

(fn GetGameSceneHUD
  (bind _ashud_game_scene (Utilities|Casting|CastToHUD_GameScene (HUD|GetHUD (Game|GetPlayerController 0)))
    (:then
      (return _ashud_game_scene))
    (:CastFailed
      (Development|PrintString 0 "Error: No active Game Scene Hud in scene." true true "(R=1.000000,G=0.000000,B=0.017078,A=1.000000)" 5.0))))

(fn GetMainMenuSceneHUD
  (bind _ashud_main_menu_scene (Utilities|Casting|CastToHUD_MainMenuScene (HUD|GetHUD (Game|GetPlayerController 0)))
    (:then
      (return _ashud_main_menu_scene))
    (:CastFailed
      (Development|PrintString 0 "Error: No active Main Menu Scene Hud in scene." true true "(R=1.000000,G=0.000000,B=0.017078,A=1.000000)" 5.0))))

(fn GetCustomGameMode
  (bind _asbp_custom_game_instance (Utilities|Casting|CastToBP_CustomGameInstance (Game|GetGameInstance))
    (:then
      _)
    (:CastFailed
      (Development|PrintString 0 "'GetCustomGameInstance' IS FAILING TO CAST TO 'BP_CustomGameInstance'. RETURNING NULL" true true "(R=1.000000,G=0.000000,B=0.054681,A=1.000000)" 1e+01)))
  (return _asbp_custom_game_instance))

(fn GetCustomGameInstance
  (bind _asbp_custom_game_instance (Utilities|Casting|CastToBP_CustomGameInstance (Game|GetGameInstance))
    (:then
      _)
    (:CastFailed
      (Development|PrintString 0 "'GetCustomGameInstance' IS FAILING TO CAST TO 'BP_CustomGameInstance'. RETURNING NULL" true true "(R=1.000000,G=0.000000,B=0.054681,A=1.000000)" 1e+01)))
  (return _asbp_custom_game_instance))

(fn GetSublevelbyName
  (params (Sublevel :type EN_Sublevels%20Enum :default "NewEnumerator2"))
  (return (Utilities|String|StringToName (Utilities|String|EnumtoString Sublevel))))