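; BP_IceElemental is an enemy AI character whose own logic is an ice wall cast.
; CastIceWall gets the current target from its BP_BaseEnemyAIController and, if valid, spawns the NS_Ice_wall Niagara effect at that target's location with random yaw.
; The cast only spawns the effect, with no damage or collision logic here.
; The construction script and melee damage collision toggle defer to the parent, and the event graph is unused.
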(event EventBeginPlay
  (|CallParentFunction) ; This node is disabled and will not be called.\nDrag off pins to build functionality.
)

(event Collision|EventActorBeginOverlap
  (params (OtherActor :type Actor%20Object%20Reference)))

(event EventTick
  (params (DeltaSeconds :type Float%20%28single-precision%29))
  (|CallParentFunction DeltaSeconds) ; This node is disabled and will not be called.\nDrag off pins to build functionality.
)

(fn ConstructionScript
  (|CallParentFunction))

(fn ToggleMeleeDamageCollision
  (params (IsEnabled :type Boolean) (CollisionIndex :type Integer))
  (|CallParentFunction IsEnabled CollisionIndex))

(fn CastIceWall
  (bind _asbp_base_enemy_aicontroller (Utilities|Casting|CastToBP_BaseEnemyAIController (AI|GetAIController 0)))
  (Utilities|IsValid (Default|GetTarget _asbp_base_enemy_aicontroller)
    (:Is%20Valid
      (Niagara|SpawnSystematLocation "/Game/Assets/VFX/StylizedToonVFX3/Effects/NS_Ice_wall.NS_Ice_wall" (Transformation|GetActorLocation (Default|GetTarget _asbp_base_enemy_aicontroller)) (Math|Rotator|MakeRotator 0.0 0.0 (Math|Random|RandomFloatinRange 0.0 3.6e+02))))))