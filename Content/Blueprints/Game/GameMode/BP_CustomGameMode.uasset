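; Game mode that boots a level, spawns the player at the current checkpoint and restarts the level on death.
; BeginPlay starts music, loads sublevels by checkpoint ID (only checkpoint 0 is implemented), loads saved settings and notifies the HUD.
; Spawning falls back from checkpoint to PlayerStart to world origin.
; Player death or destruction triggers one delayed reload for the HUD fade, forcing this game mode through level options.
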(event Custom|OnDestroyed_Event
  (params (DestroyedActor :type Actor%20Object%20Reference))
  ;[1 1 1] Reload Level On Death
  (if (not (Variables|Default|Get_isCharacterDead))
    (Variables|Default|Set_isCharacterDead true)
    (Utilities|FlowControl|Delay (Variables|Default|Get_restartLevelAfterSeconds)) ; Add a delay so the HUD can perform a fade out
    (bind _returnvalue (Game|GetCurrentLevelName true))
    (Game|OpenLevel(byName) (Utilities|String|StringToName _returnvalue) true "?Game=/Game/Blueprints/Game/GameMode/BP_CustomGameMode.BP_CustomGameMode_C") ; Forces this game mode in options
  ))

(event Custom|OnDeathComplete_Event_0
  ;[1 1 1] Reload Level On Death
  (if (not (Variables|Default|Get_isCharacterDead))
    (Variables|Default|Set_isCharacterDead true)
    (Utilities|FlowControl|Delay (Variables|Default|Get_restartLevelAfterSeconds)) ; Add a delay so the HUD can perform a fade out
    (bind _returnvalue (Game|GetCurrentLevelName true))
    (Game|OpenLevel(byName) (Utilities|String|StringToName _returnvalue) true "?Game=/Game/Blueprints/Game/GameMode/BP_CustomGameMode.BP_CustomGameMode_C") ; Forces this game mode in options
  ))

(event EventBeginPlay
  (bind __baseplayercharacter (Variables|Default|Get_basePlayerCharacter))
  (Default|PlayMusic (CallFunction|GetCustomGameInstance) "/Game/Audio/Music/POL-chubby-cat-short.POL-chubby-cat-short" 1.0 2.0)
  ;[1 1 1] Setup which levels to load on start up
  (|LevelLoadGraph
    (:%20
      ;[1 1 1] Initialize Game, create player and setup listeners
      (CallFunction|InitializeGame (Variables|Default|Get_playerClass))
      (Utilities|FlowControl|Sequence
        (:then_0
          ;[1 1 1] Reload Level On Death
          (EventDispatchers|AssignOnDeathComplete __baseplayercharacter (delegate Custom|OnDeathComplete_Event_0))
          (Game|AssignOnDestroyed __baseplayercharacter (delegate Custom|OnDestroyed_Event)) ; Incase a student didn't follow instructions\nand is just destroying the player; \nwe'll still reload the level
        )))))

(fn ConstructionScript)

(fn InitializeGame
  (params (PlayerClass :type Actor%20Class%20Reference))
  (bind (_spawnlocation _spawnrotation) (CallFunction|GetValidCharacterSpawnPoint))
  (bind _customgameinstance (CallFunction|GetCustomGameInstance))
  (Utilities|IsValid _customgameinstance
    (:Is%20Valid
      (CallFunction|SetCheckpoints)
      (Default|LoadGameStateSettings _customgameinstance)
      (CallFunction|CreatePlayerCharacter PlayerClass _spawnlocation _spawnrotation)
      (Default|OnGameInitialized (CallFunction|GetGameSceneHUD)))))

(fn SetCheckpoints
  (Utilities|Array|Clear (Variables|Default|Get_checkpoints))
  (bind _outactors (Actor|GetAllActorsOfClass "/Game/Blueprints/Game/Checkpoint/BP_Checkpoint.BP_Checkpoint_C"))
  (bind _output_get (Variables|Default|Set_checkpoints _outactors))
  (return _output_get))

(fn CreatePlayerCharacter
  (params (Class :type Actor%20Class%20Reference) (Spawn%20Transform%20Location :type Vector) (Spawn%20Transform%20Rotation :type Rotator))
  (bind _returnvalue (Game|SpawnActorfromClass Class (Math|Transform|MakeTransform Spawn%20Transform%20Location Spawn%20Transform%20Rotation "1.000000,1.000000,1.000000") "Undefined" "SelectDefaultAtRuntime" 0 0))
  (bind _asbp_base_player_character (Utilities|Casting|CastToBP_BasePlayerCharacter _returnvalue)
    (:then
      (bind _output_get (Variables|Default|Set_basePlayerCharacter _asbp_base_player_character))
      (return _output_get))
    (:CastFailed
      (Development|PrintString (Utilities|String|Append "ERROR: The requested player class '" (Utilities|GetClassDisplayName Class) "' does not implent from 'BP_BasePlayerCharacter'") true true "(R=0.244792,G=0.000000,B=0.002922,A=1.000000)" 1e+01))))

(fn GetCheckpoint
  (params (ID :type Integer))
  (bind _array_element (Utilities|Array|ForEachLoopwithBreak (Variables|Default|Get_checkpoints))
    (:LoopBody
      (if (== (Default|GetID _array_element) ID)
        (return _array_element)))))

(fn GetValidCharacterSpawnPoint
  (bind _id (CallFunction|GetCurrentCheckpointID))
  (bind _checkpoint (CallFunction|GetCheckpoint _id))
  (bind _returnvalue (Transformation|GetActorTransform _checkpoint))
  (Utilities|IsValid _checkpoint
    (:Is%20Valid
      ;[1 1 1] Return checkpoint info
      (LocalVariables|Set_spawnRotation (.rotation _returnvalue))
      (LocalVariables|Set_spawnLocation (.location _returnvalue)))
    (:Is%20Not%20Valid
      (bind _outactors (Actor|GetAllActorsOfClass "/Script/Engine.PlayerStart")) ; If no checkpoint, search for a player start
      (for _array_element _outactors
        (Utilities|IsValid _array_element
          (:Is%20Valid
            (LocalVariables|Set_spawnLocation (.location (Transformation|GetActorTransform _array_element)))
            (LocalVariables|Set_spawnRotation (.rotation (Transformation|GetActorTransform _array_element)))
            (return (LocalVariables|Get_spawnLocation) (LocalVariables|Get_spawnRotation)))))
      ;[1 1 1] If no checkpoint id or player start, return center of map
      (LocalVariables|Set_spawnRotation "0, 0, 0")
      (LocalVariables|Set_spawnLocation "0, 0, 0")))
  (return (LocalVariables|Get_spawnLocation) (LocalVariables|Get_spawnRotation)))